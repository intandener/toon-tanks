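; BP_TankGameModeBase is the tank game mode Blueprint that handles the UI for match start, turret objective and match end.
; GameStart creates the objective widget with the alive turret count, plus a start widget given the start delay.
; OnAliveTurretsChanged stores the new count and refreshes the objective text.
; GameOver shows an end widget set with whether the player won.
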(event EventOnAliveTurretsChanged
  (params (NumTurretsAlive :type Integer))
  (bind _output_get (Variables|Default|SetNumAliveTurrets NumTurretsAlive))
  (Variables|/Game/Blueprints/Widgets/WBP_Objective.WBP_Objective_C|SetAliveTurrets (Variables|Default|GetObjectiveWidget) _output_get)
  (Default|UpdateText (Variables|Default|GetObjectiveWidget)))

(event EventGameStart
  (Utilities|FlowControl|Sequence
    (:then_0
      (bind _returnvalue (UserInterface|CreateWidget "/Game/Blueprints/Widgets/WBP_Objective.WBP_Objective_C"))
      (bind _output_get (Variables|Default|SetObjectiveWidget _returnvalue))
      (Variables|/Game/Blueprints/Widgets/WBP_Objective.WBP_Objective_C|SetAliveTurrets _output_get (Variables|Default|GetNumAliveTurrets))
      (Default|UpdateText (Variables|Default|GetObjectiveWidget))
      (UserInterface|Viewport|AddtoViewport _output_get 0))
    (:then_1
      (bind _returnvalue_2 (UserInterface|CreateWidget "/Game/Blueprints/Widgets/WBP_GameStart.WBP_GameStart_C"))
      (Default|SetStartDelay _returnvalue_2 (Variables|Default|GetStartDelay))
      (UserInterface|Viewport|AddtoViewport _returnvalue_2 0))))

(event EventGameOver
  (params (bPlayerWon :type Boolean))
  (bind _returnvalue (UserInterface|CreateWidget "/Game/Blueprints/Widgets/WBP_GameEnd.WBP_GameEnd_C"))
  (Default|SetPlayerWon _returnvalue bPlayerWon)
  (UserInterface|Viewport|AddtoViewport _returnvalue 0))

(fn ConstructionScript)